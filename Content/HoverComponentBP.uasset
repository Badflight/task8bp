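; Scene component that provides hover suspension at its location on an owning HoverVehicleBP.
; Each tick it traces along its down vector up to HoverDistance, with debug drawing, to measure compression.
; On a hit, a spring-damper force along its up vector is applied to the vehicle's root primitive at the component's location.
; Damping uses the change in compression since the last hit, divided by delta time.
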(event `self.ReceiveBeginPlay`
  (bind _ashover_vehicle_bp (cast `/Game/HoverVehicleBP` (`self.GetOwner`)))
  (set `self.ParentVehicle` _ashover_vehicle_bp))

(event `self.ReceiveTick`
  (params (DeltaSeconds :type "Float (single-precision)"))
  (bind _returnvalue (`self.K2_GetComponentLocation`))
  (`/Engine/EditorBlueprintResources/StandardMacros.IsValid` (`self.ParentVehicle`)
    (:`Is Valid`
      (bind (_outhit _returnvalue_2) (`KismetSystemLibrary.LineTraceSingle` :`Start` _returnvalue :`End` (- _returnvalue (* (`self.GetUpVector`) (`self.HoverDistance`))) :`TraceChannel` "TraceTypeQuery1" :`DrawDebugType` "ForOneFrame"))
      (if _returnvalue_2
        (bind _output_get (set `self.HoverDelta` (- (`self.HoverDistance`) (`.Distance` (`GameplayStatics.BreakHitResult` _outhit)))))
        (`PrimitiveComponent.AddForceAtLocation` (cast `PrimitiveComponent` (`Actor.RootComponent` (`self.ParentVehicle`)) :!pure true) (* (`self.GetUpVector`) (+ (* (/ (- _output_get (`self.PreviouseDelta`)) (`GameplayStatics.GetWorldDeltaSeconds`)) (`self.DampingCoefficent`)) (* _output_get (`self.SpringCoefficent`)))) (`self.K2_GetComponentLocation`) "None")
        (set `self.PreviouseDelta` (`self.HoverDelta`))))))